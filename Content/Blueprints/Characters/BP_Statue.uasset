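; BP_Statue is a stalking statue character that pursues the player only while unseen, in Weeping Angel style.
; Each tick CheckIfSeen combines a camera view-cone angle test with a visibility trace from the statue's head to the camera.
; When seen it halts movement and audio; otherwise it faces the player, calls AIMoveTo and self-loops its movement sound.
; Ondeath returns it to the location saved at BeginPlay.
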(event `self.ReceiveBeginPlay`
  ;[1 1 1] On start set respawn position
  (set `self.SpawnPosition` (`self.K2_GetActorLocation`)))

(event `On death`
  ;[1 1 1] On death or kill respawn
  (`self.K2_SetActorLocation` (`self.SpawnPosition`)))

(event `Replay`
  (bind _audio (`self.Audio`))
  ;[1 1 1] Play and stop movement sound
  (`AudioComponent.Play` _audio 0.0 :!label _label)
  (add `AudioComponent.OnAudioFinished` _audio (delegate `Replay`)))

(event `self.ReceiveTick`
  (params (DeltaSeconds :type "Float (single-precision)"))
  (bind _audio (`self.Audio`))
  (bind _returnvalue (`self.K2_GetActorLocation` (`GameplayStatics.GetPlayerPawn` 0)))
  ;[1 1 1] Move and rotate if not seen
  (bind _seen (`self.checkIfSeen`))
  (if _seen
    (`Controller.StopMovement` (`AIBlueprintHelperLibrary.GetAIController` self))
    ;[1 1 1] Play and stop movement sound
    (`AudioComponent.Stop` _audio)
    (set `self.Playing` false)
    (else
      (`self.K2_SetActorRotation` (`KismetMathLibrary.FindLookAtRotation` (`self.K2_GetActorLocation`) _returnvalue))
      (`|AIMoveTo` self _returnvalue null 30.0 true
        (:`then`
          (`SceneComponent.K2_SetRelativeLocation` _audio (0.0 0.0 0.0) false false)
          (if (not (`self.Playing`))
            (set `self.Playing` true)
            (goto _label)))))))

(fn `checkIfSeen`
  (returns (Seen :type Boolean))
  (bind _returnvalue (`GameplayStatics.GetPlayerCameraManager` 0))
  (bind _returnvalue_2 (`self.K2_GetActorLocation` _returnvalue))
  ;[1 1 1] Get angle between player and statue
  (bind _angle (`self.getAngle` (- (`self.K2_GetActorLocation`) _returnvalue_2) (`self.GetActorForwardVector` _returnvalue)))
  ;[1 1 1] If within range of vision, linetrace to check obstruction
  (if (and (>= _angle -50.0) (<= _angle 50.0))
    (bind (_outhit _returnvalue_3) (`KismetSystemLibrary.LineTraceSingle` (`SceneComponent.K2_GetComponentLocation` (`self.HeadRaycast`)) _returnvalue_2 "TraceTypeQuery1"))
    (return (not _returnvalue_3))
    (else
      (return false))))

(fn `getAngle`
  (params (Vector1 :type "Vector Structure") (`Vector 2` :type "Vector Structure"))
  (returns (Angle :type "Float (double-precision)"))
  (return (`KismetMathLibrary.DegAcos` (`KismetMathLibrary.Dot_VectorVector` (`KismetMathLibrary.Normal` Vector1) (`KismetMathLibrary.Normal` `Vector 2`)))))

(fn `UserConstructionScript`)