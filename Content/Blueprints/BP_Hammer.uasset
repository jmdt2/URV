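; BP_Hammer is a hammer or mace weapon that kills statues when it strikes them mid-swing.
; Each tick it derives the Head component's speed from its change in world position and sets a Swinging flag above a speed threshold.
; On Hit, it calls OnDeath on a BP_Statue only while that flag is set, so slow contact does no harm.
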(event `self.ReceiveTick`
  (params (DeltaSeconds :type "Float (single-precision)"))
  (bind _returnvalue (`SceneComponent.K2_GetComponentLocation` (`self.Head`)))
  ;[1 1 1] Get distance to last position
  ;[1 1 1] Check if player is swinging the hammer/mace and update last position
  (set `self.Swinging` (>= (/ (`KismetMathLibrary.VSize` (- _returnvalue (`self.LastHeadPosition`))) DeltaSeconds) 1000.0))
  (set `self.LastHeadPosition` _returnvalue))

(event `self.ReceiveHit`
  (params (MyComp :type "PrimitiveComponent Object Reference") (Other :type "Actor Object Reference") (OtherComp :type "PrimitiveComponent Object Reference") (bSelfMoved :type Boolean) (HitLocation :type "Vector Structure") (HitNormal :type "Vector Structure") (NormalImpulse :type "Vector Structure") (Hit :type "HitResult Structure (by ref)"))
  ;[1 1 1] On hit, kill statue if swinging
  (if (and (`KismetMathLibrary.ClassIsChildOf` (`GameplayStatics.GetObjectClass` Other) "/Game/Blueprints/Characters/BP_Statue.BP_Statue_C") (`self.Swinging`))
    (bind _asbp_statue (cast `/Game/Blueprints/Characters/BP_Statue` Other))
    (`/Game/Blueprints/Characters/BP_Statue.On death` _asbp_statue)))

(fn `UserConstructionScript`)